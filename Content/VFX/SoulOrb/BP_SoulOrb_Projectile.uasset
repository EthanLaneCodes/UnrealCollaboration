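; Soul Orb projectile Blueprint that damages whatever it hits and then destroys itself.
; Its box collision hit event fires the OnProjectileImpact dispatcher, then sends a damage message to the hit actor with the instigator as causer.
; The impulse only launches upward, as the knockback term multiplies a zero vector.
; Each hit also plays a world camera shake and spawns an effect system at the hit location.
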(event OnComponentHit(BoxCollision)
  (params (HitComponent :type Primitive%20Component%20Object%20Reference) (OtherActor :type Actor%20Object%20Reference) (OtherComp :type Primitive%20Component%20Object%20Reference) (NormalImpulse :type Vector :default "0, 0, 0") (Hit :type Hit%20Result%20Structure%20%28by%20ref%29))
  (bind (_bblockinghit _binitialoverlap _time _distance _location _impactpoint _normal _impactnormal _physmat _hitactor) (Collision|BreakHitResult Hit))
  (Default|CallOnProjectileImpact OtherActor Hit)
  (Class|BPIDamageable|ApplyDamage(Message) _hitactor (Variables|Default|GetProjectile%20Damage) (Game|GetInstigator) _impactpoint (+ (* "" (* (Variables|Default|GetMelee%20Knockback%20Impulse) -1.0)) (* (Math|Vector|VectorUp) (Variables|Default|GetMelee%20Launch%20Impulse))))
  (Camera|PlayWorldCameraShake "/Game/Variant_Combat/Blueprints/BP_CameraShake_Hit_Enemy.BP_CameraShake_Hit_Enemy_C" "0, 0, 0" 5e+02 1e+03)
  (Niagara|SpawnSystematLocation (Variables|Effects|GetSystem%20Template) _location)
  (Actor|DestroyActor))

(event EventBeginPlay)

(event Collision|EventActorBeginOverlap
  (params (OtherActor :type Actor%20Object%20Reference)))

(event EventTick
  (params (DeltaSeconds :type Float%20%28single-precision%29)))

(fn ConstructionScript)